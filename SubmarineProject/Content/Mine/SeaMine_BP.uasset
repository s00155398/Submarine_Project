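; Sea mine actor that explodes when hit by the player or when torpedo hits deplete its health.
; Mesh hit events sort colliders by actor tag, and torpedoes subtract their radial force component's DestructibleDamage from CurrentHealth.
; Tick polls health and triggers Explode at zero or below.
; Explode spawns a particle effect, hides the point light, fires a radial force impulse and destroys the actor.
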(event OnComponentHit(StaticMesh)
  (params (HitComponent :type Primitive%20Component%20Object%20Reference) (OtherActor :type Actor%20Object%20Reference) (OtherComp :type Primitive%20Component%20Object%20Reference) (NormalImpulse :type Vector :default "0, 0, 0") (Hit :type Hit%20Result%20Structure%20%28by%20ref%29))
  (if (Actor|ActorHasTag OtherActor "Torpedo")
    (CallFunction|HandleCollisionwithTorpedo OtherActor)
    (elif (Actor|ActorHasTag OtherActor "Player")
      (CallFunction|Explode))))

(event EventTick
  (params (DeltaSeconds :type Float%20%28single-precision%29))
  (if (<= (Variables|Default|GetCurrentHealth) 0.0)
    (CallFunction|Explode)))

(fn ConstructionScript)

(fn Explode
  (Effects|SpawnEmitteratLocation "/Game/ParticleEffects/P_Explosion.P_Explosion" (Transformation|GetActorLocation self))
  (Rendering|SetVisibility (Variables|Default|GetPointLight) false false)
  (Class|RadialForceComponent|FireImpulse (Variables|Default|GetExplosion%20Force))
  (Actor|DestroyActor))

(fn HandleCollisionwithTorpedo
  (params (Object :type Object%20Object%20Reference))
  (bind _astorpedo_bp (Utilities|Casting|CastToTorpedo_BP Object))
  (Variables|Default|SetCurrentHealth (- (Variables|Default|GetCurrentHealth) (Variables|/Script/Engine.RadialForceComponent|GetDestructibleDamage (Actor|GetComponentbyClass _astorpedo_bp "/Script/Engine.RadialForceComponent")))))