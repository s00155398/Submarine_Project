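; Player submarine that fires torpedoes, toggles its two headlights and takes damage from sea mines and torpedoes.
; Hits are routed by actor tag and subtract the other actor's RadialForce destructible damage from Health, with mines also spawning an explosion.
; Tick destroys the sub once Health runs out, and destruction opens GivenLevel.
; Overlaps with "Bound" actors switch PlaneMesh physics simulation to keep the sub within water limits.
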(event OnComponentHit(PlaneMesh)
  (params (HitComponent :type Primitive%20Component%20Object%20Reference) (OtherActor :type Actor%20Object%20Reference) (OtherComp :type Primitive%20Component%20Object%20Reference) (NormalImpulse :type Vector :default "0, 0, 0") (Hit :type Hit%20Result%20Structure%20%28by%20ref%29))
  ;[1 1 1] Handle Collision
  (if (Actor|ActorHasTag OtherActor "Mine")
    (CallFunction|HandleMineCollision OtherActor)
    (elif (Actor|ActorHasTag OtherActor "Torpedo")
      (CallFunction|HandleTorpedoCollision OtherActor))))

(event EventBeginPlay)

(event Collision|EventActorBeginOverlap
  (params (OtherActor :type Actor%20Object%20Reference))
  ;[1 1 1] Stops Sub from escaping water limits
  (if (Actor|ActorHasTag OtherActor "Bound")
    (Physics|SetSimulatePhysics (Variables|Default|GetPlaneMesh) false)))

(event EventDestroyed
  (Game|OpenLevel(byName) (Variables|Default|GetGiven%20Level)))

(event EventTick
  (params (DeltaSeconds :type Float%20%28single-precision%29))
  (if (<= (Variables|Default|GetHealth) 0.0)
    (Actor|DestroyActor)))

(event Collision|EventActorEndOverlap
  (params (OtherActor :type Actor%20Object%20Reference))
  ;[1 1 1] Stops Sub from escaping water limits
  (if (Actor|ActorHasTag OtherActor "Bound")
    (Physics|SetSimulatePhysics (Variables|Default|GetPlaneMesh) true)))

(event Input|ActionEvents|InputActionFireTorpedo
  (params (Key :type Key%20Structure))
  ;[1 1 1] Input actions
  (:Pressed
    (Class|SubmarineProjectPawn|Fire)))

(event Input|KeyboardEvents|F
  (params (Key :type Key%20Structure))
  ;[1 1 1] Input actions
  (:Released
    (CallFunction|ToggleHeadLights)))

(fn ConstructionScript)

(fn ToggleHeadLights
  (Rendering|ToggleVisibility (Variables|Default|GetHeadLight1) false))

(fn HandleMineCollision
  (params (Object :type Object%20Object%20Reference))
  (bind _assea_mine_bp (Utilities|Casting|CastToSeaMine_BP Object))
  (Variables|Default|SetHealth (- (Variables|Default|GetHealth) (Variables|/Script/Engine.RadialForceComponent|GetDestructibleDamage (Actor|GetComponentbyClass _assea_mine_bp "/Script/Engine.RadialForceComponent"))))
  (Effects|SpawnEmitteratLocation "/Game/ParticleEffects/P_Explosion.P_Explosion" (Transformation|GetActorLocation _assea_mine_bp)))

(fn HandleTorpedoCollision
  (params (Object :type Object%20Object%20Reference))
  (bind _astorpedo_bp (Utilities|Casting|CastToTorpedo_BP Object))
  (Variables|Default|SetHealth (- (Variables|Default|GetHealth) (Variables|/Script/Engine.RadialForceComponent|GetDestructibleDamage (Actor|GetComponentbyClass _astorpedo_bp "/Script/Engine.RadialForceComponent")))))