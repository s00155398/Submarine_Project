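; BP_Turret is a destructible turret with base, head and barrel components that takes damage from torpedo hits.
; On BeginPlay it passes the barrel and head to a TurretAiming component, which is set up to drive aiming.
; Hit events on all three parts route to a shared handler that checks the Torpedo tag and subtracts fixed Health.
; At zero Health it spawns a scaled explosion emitter and destroys itself.
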(event OnComponentHit(TurretBase)
  (params (HitComponent :type Primitive%20Component%20Object%20Reference) (OtherActor :type Actor%20Object%20Reference) (OtherComp :type Primitive%20Component%20Object%20Reference) (NormalImpulse :type Vector :default "0, 0, 0") (Hit :type Hit%20Result%20Structure%20%28by%20ref%29))
  (CallFunction|HandleTorpedoCollision OtherActor))

(event OnComponentHit(TurretHead)
  (params (HitComponent :type Primitive%20Component%20Object%20Reference) (OtherActor :type Actor%20Object%20Reference) (OtherComp :type Primitive%20Component%20Object%20Reference) (NormalImpulse :type Vector :default "0, 0, 0") (Hit :type Hit%20Result%20Structure%20%28by%20ref%29))
  (CallFunction|HandleTorpedoCollision OtherActor))

(event OnComponentHit(TurretBarrel)
  (params (HitComponent :type Primitive%20Component%20Object%20Reference) (OtherActor :type Actor%20Object%20Reference) (OtherComp :type Primitive%20Component%20Object%20Reference) (NormalImpulse :type Vector :default "0, 0, 0") (Hit :type Hit%20Result%20Structure%20%28by%20ref%29))
  (CallFunction|HandleTorpedoCollision OtherActor))

(event EventBeginPlay
  (Class|TurretAimingComponent|Initialise (Variables|Default|GetTurretAiming) (Variables|Default|GetTurretBarrel) (Variables|Default|GetTurretHead)))

(fn ConstructionScript)

(fn HandleTorpedoCollision
  (params (self2 :type Actor%20Object%20Reference))
  (if (Actor|ActorHasTag self2 "Torpedo")
    (Variables|Default|SetHealth (- (Variables|Default|GetHealth) 5e+01))
    (if (<= (Variables|Default|GetHealth) 0.0)
      (Effects|SpawnEmitteratLocation "/Game/ParticleEffects/P_FacilityExplosion.P_FacilityExplosion" (Transformation|GetActorLocation self) "0, 0, 0" "0.500000,0.500000,0.500000")
      (Actor|DestroyActor))))