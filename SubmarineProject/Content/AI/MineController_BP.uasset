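; AI controller for a mine that runs the MineBehaviour behavior tree on the MineData blackboard.
; On BeginPlay it sets up the blackboard, starts the tree and caches the blackboard component.
; AI perception updates write sensed actors without the "Enemy" tag to the Enemy key.
; The key is cleared when such an actor's stimulus is no longer successfully sensed.
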(event OnTargetPerceptionUpdated(AIPerception)
  (params (Actor :type Actor%20Object%20Reference) (Stimulus :type AI%20Stimulus%20Structure))
  (CallFunction|UpdateBBEnemyKey Actor Stimulus Actor))

(event EventBeginPlay
  (bind _blackboardcomponent (Class|AIController|UseBlackboard "/Game/AI/MineData.MineData"))
  (AI|RunBehaviorTree "/Game/AI/MineBehaviour.MineBehaviour")
  (Variables|Default|SetBlackBoardComponent _blackboardcomponent))

(event EventTick
  (params (DeltaSeconds :type Float%20%28single-precision%29)))

(fn ConstructionScript)

(fn UpdateBBEnemyKey
  (params (Object%20Value :type Object%20Object%20Reference) (AI%20Stimulus :type AI%20Stimulus%20Structure) (Self :type Actor%20Object%20Reference))
  (bind _blackboardcomponent (Variables|Default|GetBlackBoardComponent))
  (bind _enemy (Variables|Default|GetEnemy))
  (if (not (Actor|ActorHasTag Self "Enemy"))
    (if (.bSuccessfullySensed (Utilities|Struct|BreakAIStimulus AI%20Stimulus))
      (AI|Components|Blackboard|SetValueasObject _blackboardcomponent _enemy Object%20Value)
      (else
        (AI|Components|Blackboard|ClearValue _blackboardcomponent _enemy)))))